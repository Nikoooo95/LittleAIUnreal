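; Behavior tree service that switches an NPC between following a character inside a zone and moving along its patrol positions.
; On activation it caches the first BP_CharacterController and NPC_Controller actors found in the level.
; Each tick, if the character controller's CharactersInside has an entry, it sets Following and writes that character's location to TargetPoint.
; Otherwise it clears Following and targets the NPC controller's next position.
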(event EventTick
  (params (OwnerActor :type Actor%20Object%20Reference) (DeltaSeconds :type Float%20%28single-precision%29))
  (bind _npc_controller_reference (Variables|Default|GetNPC_Controller_Reference))
  ;[1 1 1] Comprobación Continua de Personajes en la zona
  (if (Utilities|Array|IsValidIndex (Variables|/Game/BluePrints/AI/BP_CharacterController.BP_CharacterController_C|GetCharactersInside (Variables|Default|GetBP_Controller_Reference)))
    (AI|BehaviorTree|SetBlackboardValueasVector (Variables|Default|GetTargetPoint) (Transformation|GetActorLocation (Utilities|Array|Get(acopy) (Variables|/Game/BluePrints/AI/BP_CharacterController.BP_CharacterController_C|GetCharactersInside (Variables|Default|GetBP_Controller_Reference)))))
    (Class|BTFunctionLibrary|SetBlackboardValueasBool (Variables|Default|GetFollowing) true)
    (else
      (Class|BTFunctionLibrary|SetBlackboardValueasBool (Variables|Default|GetFollowing) false)
      (AI|BehaviorTree|SetBlackboardValueasVector (Variables|Default|GetTargetPoint) (Transformation|GetActorLocation (Utilities|Array|Get(acopy) (Variables|/Game/BluePrints/AI/NPC_Controller.NPC_Controller_C|GetPositions _npc_controller_reference) (Variables|/Game/BluePrints/AI/NPC_Controller.NPC_Controller_C|GetNextPosition _npc_controller_reference)))))))

(event EventReceiveActivation
  (params (OwnerActor :type Actor%20Object%20Reference))
  ;[1 1 1] Activacion Del Servicio
  (bind _outactors (Actor|GetAllActorsOfClass "/Game/BluePrints/AI/BP_CharacterController.BP_CharacterController_C"))
  (Variables|Default|SetBP_Controller_Reference (Utilities|Array|Get(acopy) _outactors))
  (bind _outactors_2 (Actor|GetAllActorsOfClass "/Game/BluePrints/AI/NPC_Controller.NPC_Controller_C"))
  (Variables|Default|SetNPC_Controller_Reference (Utilities|Array|Get(acopy) _outactors_2)))