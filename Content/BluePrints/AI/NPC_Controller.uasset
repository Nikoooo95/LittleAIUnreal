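; AI controller for an NPC that patrols a looping waypoint route unless its blackboard flags it as following.
; BeginPlay gathers Route_Waypoint_0 actors, seeds the blackboard's TargetPoint with the first, takes the first NPC_AI found and runs Behaviour_Tree_AI.
; While not following, Tick uses a tolerance-based distance check to advance and wrap the waypoint index, without rewriting TargetPoint.
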(event EventBeginPlay
  ;[1 1 1] Recoge a los personajes
  (bind _outactors (Actor|GetAllActorsOfClass "/Game/BluePrints/ControlledObject.ControlledObject_C"))
  (Variables|Arrays|SetCharacters%20Controller _outactors)
  (Class|AIController|UseBlackboard "/Game/BluePrints/AI/Data_AI.Data_AI")
  (Utilities|FlowControl|Sequence
    (:then_0
      ;[1 1 1] Encuentra las posiciones y pasale la primera
      (bind _outactors_2 (Actor|GetAllActorsOfClass "/Game/BluePrints/AI/Route_Waypoint_0.Route_Waypoint_0_C"))
      (for _array_element _outactors_2
        (Utilities|Array|Add (Variables|Arrays|GetPositions) _array_element)
        (AI|Components|Blackboard|SetValueasVector (AI|GetBlackboard self) (Variables|Names|GetTargetPoint) (Transformation|GetActorLocation (Utilities|Array|Get(acopy) (Variables|Arrays|GetPositions) (Variables|Int|GetNextPosition))))))
    (:then_1
      ;[1 1 1] Recoge al personaje y ejecuta el Behaviour Tree
      (bind _outactors_3 (Actor|GetAllActorsOfClass "/Game/BluePrints/AI/NPC_AI.NPC_AI_C"))
      (Variables|References|SetNPC_Reference (Utilities|Array|Get(acopy) _outactors_3))
      (AI|RunBehaviorTree "/Game/BluePrints/AI/Behaviour_Tree_AI.Behaviour_Tree_AI"))))

(event EventTick
  (params (DeltaSeconds :type Float%20%28single-precision%29))
  ;[1 1 1] Sigue a alguien?
  (Variables|Bool|SetFollowing (ScalableFloat|GetValueasBool (AI|GetBlackboard self) (Variables|Names|GetFollowingName)))
  (if (not (Variables|Bool|GetFollowing))
    ;[1 1 1] Está cerca de la siguiente posicion?
    (bind _result (CallFunction|NearlyEqual (Transformation|GetActorLocation (Variables|References|GetNPC_Reference)) (Transformation|GetActorLocation (Utilities|Array|Get(acopy) (Variables|Arrays|GetPositions) (Variables|Int|GetNextPosition))) (Variables|Float|GetTolerancy)))
    (if _result
      ;[1 1 1] Calcula la siguiente posición
      (if (< (Variables|Int|GetNextPosition) (- (Utilities|Array|Length (Variables|Arrays|GetPositions)) 1))
        (Variables|Int|SetNextPosition (+ (Variables|Int|GetNextPosition) 1))
        (else
          (Variables|Int|SetNextPosition 0))))))

(fn ConstructionScript)

(fn NearlyEqual
  (params (Vector1 :type Vector) (Vector2 :type Vector) (Tolerancia :type Float%20%28single-precision%29))
  ;[1 1 1] Comprobación Si Esta Cerca
  (return (<= (Math|Float|Absolute(Float) (Math|Vector|VectorLength (- Vector1 Vector2))) Tolerancia)))